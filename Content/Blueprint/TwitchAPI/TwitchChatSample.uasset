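; Sample Twitch integration actor that connects to chat, prints incoming messages and registers a "fire" command, with a handler that spawns bullets through BP_BulletSpawner.
; On BeginPlay it loads saved TwitchConfig credentials and validates the token, falling back to the authentication component's Init.
; A new token triggers a user info fetch with a hardcoded username, then chat connection and saving to the TwitchSettings slot.
; Construction links TwitchPubSub to authentication as its EventSub component.
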(event OnTokenReceived(TwitchAuthentication)
  (params (token :type String))
  (bind _twitchauthentication (Variables|Default|GetTwitchAuthentication))
  (Class|TwitchAuthentication|FetchUserInfo _twitchauthentication "zeplin455" token)
  (Variables|Default|SetAuthToken token)
  (Variables|/Script/TwitchInteraction.TwitchAuthentication|Settoken _twitchauthentication token))

(event OnUserIdReceived(TwitchAuthentication)
  (params (userId :type String))
  (bind _twitchchat (Variables|Default|GetTwitchChat))
  (bind _twitchauthentication (Variables|Default|GetTwitchAuthentication))
  (bind _twitchauthentication_2 (Variables|Default|GetTwitchAuthentication))
  (bind _username (Variables|/Script/TwitchInteraction.TwitchAuthentication|Getusername _twitchauthentication))
  (Class|TwitchChat|SetUserInfo _twitchchat (Variables|Default|GetAuthToken) "oauth" _username _username)
  (bind (_result _returnvalue) (Class|TwitchChat|Connect _twitchchat))
  (if _returnvalue
    (Development|PrintString _result)
    (bind __result (Class|TwitchChat|AuthenticateTwitchChat (Variables|Default|GetTwitchChat)))
    (Development|PrintString __result)
    (Development|PrintString "Connected to chat")
    (bind _returnvalue_2 (SaveGame|CreateSaveGameObject "/TwitchInteractionUE/Examples/State/TwitchConfig.TwitchConfig_C"))
    (Variables|/TwitchInteractionUE/Examples/State/TwitchConfig.TwitchConfig_C|SetTwitchChannelId _returnvalue_2 (Variables|/Script/TwitchInteraction.TwitchAuthentication|Getuserid _twitchauthentication_2))
    (Variables|/TwitchInteractionUE/Examples/State/TwitchConfig.TwitchConfig_C|SetTwitchClientId _returnvalue_2 (Variables|/Script/TwitchInteraction.TwitchAuthentication|GetclientId _twitchauthentication_2))
    (Variables|/TwitchInteractionUE/Examples/State/TwitchConfig.TwitchConfig_C|SetTwitchListenPort _returnvalue_2 (Variables|/Script/TwitchInteraction.TwitchAuthentication|GetlistenPort _twitchauthentication_2))
    (Variables|/TwitchInteractionUE/Examples/State/TwitchConfig.TwitchConfig_C|SetTwitchRedirectUrl _returnvalue_2 (Variables|/Script/TwitchInteraction.TwitchAuthentication|GetredirectUrl _twitchauthentication_2))
    (Variables|/TwitchInteractionUE/Examples/State/TwitchConfig.TwitchConfig_C|SetTwitchToken _returnvalue_2 (Variables|/Script/TwitchInteraction.TwitchAuthentication|Gettoken _twitchauthentication_2))
    (Variables|/TwitchInteractionUE/Examples/State/TwitchConfig.TwitchConfig_C|SetTwitchUsername _returnvalue_2 (Variables|/Script/TwitchInteraction.TwitchAuthentication|Getusername _twitchauthentication_2))
    (SaveGame|SaveGametoSlot _returnvalue_2 "TwitchSettings")))

(event OnTokenValidReceived(TwitchAuthentication)
  (params (success :type Boolean))
  (bind _twitchchat (Variables|Default|GetTwitchChat))
  (bind _twitchauthentication (Variables|Default|GetTwitchAuthentication))
  (bind _username (Variables|/Script/TwitchInteraction.TwitchAuthentication|Getusername _twitchauthentication))
  (if success
    (Class|TwitchChat|SetUserInfo _twitchchat (Variables|Default|GetAuthToken) "oauth" _username _username)
    (bind (_result _returnvalue) (Class|TwitchChat|Connect _twitchchat))
    (if _returnvalue
      (Development|PrintString _result)
      (Development|PrintString "Connected to Twitch chat")
      (bind __result (Class|TwitchChat|AuthenticateTwitchChat (Variables|Default|GetTwitchChat)))
      (Development|PrintString __result)
      (else
        (Development|PrintString "Failed to connect to twitch chat")))
    (else
      (Class|TwitchAuthentication|Init _twitchauthentication))))

(event OnMessageReceived(TwitchChat)
  (params (message :type Twitch%20Irc%20Message%20Structure%20%28by%20ref%29))
  (bind (_badgeinfo _badges _color _displayname _emotes _flags _id _mod _roomid _subscriber _messagetimestamp _turbo _userid _usertype _userirclogin _messagetype _channelname _bits _message) (Utilities|Struct|BreakTwitchIrcMessage message))
  (Development|PrintString (Utilities|String|Append _displayname " : " _message)))

(event Custom|ViewFiring
  (params (commandName :type String) (commandOptions :type Array%20of%20Strings) (senderUsername :type String))
  (bind _returnvalue (Actor|GetActorOfClass "/Game/Blueprint/Bullet/BP_BulletSpawner.BP_BulletSpawner_C"))
  (Utilities|IsValid _returnvalue
    (:Is%20Valid
      (Default|SpawnBullet _returnvalue))))

(event EventBeginPlay
  (bind _twitchauthentication (Variables|Default|GetTwitchAuthentication))
  (Class|TwitchChat|RegisterCommand (Variables|Default|GetTwitchChat) "fire" (EventDispatchers|CreateEvent :!event Custom|ViewFiring))
  (bind _returnvalue (SaveGame|LoadGamefromSlot "TwitchSettings"))
  (bind _astwitch_config (Utilities|Casting|CastToTwitchConfig _returnvalue)
    (:then
      (Variables|/Script/TwitchInteraction.TwitchAuthentication|SetlistenPort _twitchauthentication (Variables|/TwitchInteractionUE/Examples/State/TwitchConfig.TwitchConfig_C|GetTwitchListenPort _astwitch_config))
      (Variables|/Script/TwitchInteraction.TwitchAuthentication|SetredirectUrl _twitchauthentication (Variables|/TwitchInteractionUE/Examples/State/TwitchConfig.TwitchConfig_C|GetTwitchRedirectUrl _astwitch_config))
      (Variables|/Script/TwitchInteraction.TwitchAuthentication|Setuserid _twitchauthentication (Variables|/TwitchInteractionUE/Examples/State/TwitchConfig.TwitchConfig_C|GetTwitchChannelId _astwitch_config))
      (Variables|/Script/TwitchInteraction.TwitchAuthentication|Setusername _twitchauthentication (Variables|/TwitchInteractionUE/Examples/State/TwitchConfig.TwitchConfig_C|GetTwitchUsername _astwitch_config))
      (Variables|/Script/TwitchInteraction.TwitchAuthentication|SetclientId _twitchauthentication (Variables|/TwitchInteractionUE/Examples/State/TwitchConfig.TwitchConfig_C|GetTwitchClientId _astwitch_config))
      (Variables|Default|SetAuthToken (Variables|/TwitchInteractionUE/Examples/State/TwitchConfig.TwitchConfig_C|GetTwitchToken _astwitch_config))
      (Variables|/Script/TwitchInteraction.TwitchAuthentication|Settoken _twitchauthentication (Variables|/TwitchInteractionUE/Examples/State/TwitchConfig.TwitchConfig_C|GetTwitchToken _astwitch_config))
      (Class|TwitchAuthentication|CheckTokenValid _twitchauthentication))
    (:CastFailed
      (Class|TwitchAuthentication|Init (Variables|Default|GetTwitchAuthentication)))))

(event Collision|EventActorBeginOverlap
  (params (OtherActor :type Actor%20Object%20Reference)))

(event EventTick
  (params (DeltaSeconds :type Float%20%28single-precision%29)))

(fn ConstructionScript
  (Variables|/Script/TwitchInteraction.TwitchAuthentication|SetEventSubComponent (Variables|Default|GetTwitchAuthentication) (Variables|Default|GetTwitchPubSub)))